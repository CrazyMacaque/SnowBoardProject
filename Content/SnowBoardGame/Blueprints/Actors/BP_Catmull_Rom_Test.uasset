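; Test actor that builds a Catmull-Rom curve from editable control points and writes it to a Spline component.
; The construction script converts the points to world space, samples the curve at even steps with a Γ parameter, then sets the spline points.
; Sampling covers three segments across four points, mirroring phantom points at both ends.
; The middle segment is appended before the first and last, so output is not in path order.
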(fn `GetCatmullRomFunctionUarray`
  (params (ControlPointsArray :type "Array of Vector Structure") (`γ` :type "Float (double-precision)"))
  (returns (UArray :type "Array of Vector Structure"))
  (bind _output (`|GetArrayItem` ControlPointsArray 3))
  (bind _output_2 (`|GetArrayItem` ControlPointsArray))
  (bind _output_3 (`|GetArrayItem` ControlPointsArray 1))
  (bind _output_4 (`|GetArrayItem` ControlPointsArray 2))
  (bind _alpha (`self.Alpha`))
  (bind _returnvalue (`KismetMathLibrary.MakeVector` _alpha _alpha _alpha))
  (for _ (range (`self.Last Index`))
    (bind _curvepoint (`/Game/SnowBoardGame/Blueprints/FunctionLibrary/BPF_Catmull_RomCurve.GetCatmullRom` _output_2 _output_3 _output_4 _output `γ` _returnvalue))
    (`KismetArrayLibrary.Array_Add` (`self.MidCurveUArray`) _curvepoint)
    (set `self.Alpha` (+ (`self.Alpha`) (/ 1.0 (`KismetMathLibrary.Conv_IntToDouble` (`self.Last Index`))))))
  (set `self.Alpha` 0.0)
  (for _ (range (`self.Last Index`))
    (bind _curvepoint_2 (`/Game/SnowBoardGame/Blueprints/FunctionLibrary/BPF_Catmull_RomCurve.GetCatmullRom` (- (* _output_2 2.0) _output_3) _output_2 _output_3 _output_4 `γ` _returnvalue))
    (`KismetArrayLibrary.Array_Add` (`self.MidCurveUArray`) _curvepoint_2)
    (set `self.Alpha` (+ (`self.Alpha`) (/ 1.0 (`KismetMathLibrary.Conv_IntToDouble` (`self.Last Index`))))))
  (set `self.Alpha` 0.0)
  (for _ (range (`self.Last Index`))
    (bind _curvepoint_3 (`/Game/SnowBoardGame/Blueprints/FunctionLibrary/BPF_Catmull_RomCurve.GetCatmullRom` _output_3 _output_4 _output (- (* _output 2.0) _output_4) `γ` _returnvalue))
    (`KismetArrayLibrary.Array_Add` (`self.MidCurveUArray`) _curvepoint_3)
    (set `self.Alpha` (+ (`self.Alpha`) (/ 1.0 (`KismetMathLibrary.Conv_IntToDouble` (`self.Last Index`))))))
  (set `self.Alpha` 0.0)
  (return (`self.MidCurveUArray`)))

(fn `UserConstructionScript`
  (if (`self.CanUpdate`)
    (for _array_element (`self.ControlPoints`)
      (`KismetArrayLibrary.Array_Add` (`self.TempCurvePoints`) (`KismetMathLibrary.TransformLocation` (`self.GetTransform`) _array_element)))
    (bind _uarray (`self.GetCatmullRomFunctionUarray` (`self.TempCurvePoints`) (`self.γ`)))
    (for _array_element_2 _uarray
      (set `self.CanUpdate` false)
      (`KismetArrayLibrary.Array_Add` (`self.SplinePoints`) _array_element_2))
    (set `self.CanUpdate` true)
    (`SplineComponent.SetSplinePoints` (`self.Spline`) (`self.SplinePoints`) "World" true)))