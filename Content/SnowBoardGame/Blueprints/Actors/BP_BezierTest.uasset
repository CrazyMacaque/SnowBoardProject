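; BP_BezierTest is a test actor that shapes a spline along an N-order Bezier curve.
; The construction script converts CurvePoints to world space, samples BezierCurve in LastIndex-based steps and feeds the results to the spline.
; BeginPlay gathers BP_Target locations, but the timeline debug-sphere preview that would use them is disconnected.
; A quadratic variant using three control points is also left unconnected.
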(event `self.ReceiveBeginPlay`
  (bind _outactors (`GameplayStatics.GetAllActorsOfClass` "/Game/SnowBoardGame/Blueprints/Actors/BP_Target.BP_Target_C"))
  (for _array_element _outactors
    (`KismetArrayLibrary.Array_Add` (`self.BP_TargetPoints`) (`self.K2_GetActorLocation` _array_element))))

(fn `UserConstructionScript`
  ;[0.8632 0.04374 0.1144] N阶贝塞尔曲线
  (if (`self.CanDraw`)
    (for _array_element (`self.CurvePoints`)
      (`KismetArrayLibrary.Array_Add` (`self.TempCurvePoints`) (`KismetMathLibrary.TransformLocation` (`self.GetTransform`) _array_element)))
    (for _ (range (`self.Last Index`))
      (set `self.CanDraw` false)
      (bind _output (`/Game/SnowBoardGame/Blueprints/FunctionLibrary/BPF_BezierCurve.Bezier Curve` (`self.TempCurvePoints`) (`self.T`)))
      (set `self.T` (+ (`self.T`) (/ 1.0 (`KismetMathLibrary.Conv_IntToDouble` (`self.Last Index`)))))
      (`KismetArrayLibrary.Array_Add` (`self.SplinePoints`) _output))
    (set `self.CanDraw` true)
    (`SplineComponent.SetSplinePoints` (`self.Spline`) (`self.SplinePoints`) "World" true)))