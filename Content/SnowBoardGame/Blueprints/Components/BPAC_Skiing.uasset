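; Skiing ability component for the snowboard game that, while active, slides the owning character over terrain by simulating forces in Flying movement mode.
; Activation and deactivation switch motion mode, movement mode, fly speed and ticking through the ability-owner interface and CharacterMovement.
; Each tick traces the floor, sums gravity, slope support, forward thrust and curve-scaled, velocity-relative steering into movement input, then eases rotation toward velocity with clamped pitch.
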(event `self.ReceiveBeginPlay`
  (`self.InitData`))

(event `self.ReceiveTick`
  (params (DeltaSeconds :type "Float (single-precision)"))
  (`|ExecutionSequence`
    (:`then_0`
      (`self.UpdateMovement`))
    (:`then_1`
      (`self.UpateCharacterState`))))

(event `/Game/SnowBoardGame/Blueprints/Interface/BPI_Ability.DoActive`
  (`self.InitSetting`))

(event `/Game/SnowBoardGame/Blueprints/Interface/BPI_Ability.DoDeactive`
  (`self.EndSetting`))

(event `/Game/SnowBoardGame/Blueprints/Interface/BPI_Ability.InputAxis`
  (params (AxisName :type "/Game/SnowBoardGame/Blueprints/Enum/EBP_InputAxisName Enum" :default "NewEnumerator0") (AxisValue :type "Float (single-precision)"))
  (switch `/Game/SnowBoardGame/Blueprints/Enum/EBP_InputAxisName` AxisName
    (:`NewEnumerator1`
      (`self.MoveForward` AxisValue))
    (:`NewEnumerator2`
      (`self.MoveRight` AxisValue))))

(fn `AddMovementInput`
  (`Pawn.AddMovementInput` (`Actor.Instigator` (`self.GetOwner`)) (`self.MovementDirection`) (`self.MoveForwardAxis`) true))

(fn `AdjustCharacterRotation`
  (`Actor.K2_SetActorRotation` (`self.GetOwner`) (`KismetMathLibrary.MakeRotator` (.roll (`KismetMathLibrary.RInterpTo` (`Actor.K2_GetActorRotation` (`self.GetOwner`)) (`KismetMathLibrary.Quat_Rotator` (`KismetMathLibrary.Conv_VectorToQuaternion` (`MovementComponent.Velocity` (`self.Character Movement`)))) (`GameplayStatics.GetWorldDeltaSeconds`) (`self.CharacterRotationInterpSpeed`))) (`KismetMathLibrary.FClamp` (.pitch (`KismetMathLibrary.RInterpTo` (`Actor.K2_GetActorRotation` (`self.GetOwner`)) (`KismetMathLibrary.Quat_Rotator` (`KismetMathLibrary.Conv_VectorToQuaternion` (`MovementComponent.Velocity` (`self.Character Movement`)))) (`GameplayStatics.GetWorldDeltaSeconds`) (`self.CharacterRotationInterpSpeed`))) -35.0 59.0) (.yaw (`KismetMathLibrary.RInterpTo` (`Actor.K2_GetActorRotation` (`self.GetOwner`)) (`KismetMathLibrary.Quat_Rotator` (`KismetMathLibrary.Conv_VectorToQuaternion` (`MovementComponent.Velocity` (`self.Character Movement`)))) (`GameplayStatics.GetWorldDeltaSeconds`) (`self.CharacterRotationInterpSpeed`)))) false))

(fn `EndSetting`
  (`|ExecutionSequence`
    (:`then_0`
      (`/Game/SnowBoardGame/Blueprints/Interface/BPI_AbilityOwner.SetMotionMode` (`self.As BPI Ability Owner`) "NewEnumerator0")
      (`CharacterMovementComponent.SetMovementMode` (`self.Character Movement`) "MOVE_Walking" 0)
      (`self.SetComponentTickEnabled` false)
      (set `CharacterMovementComponent.MaxFlySpeed` (`self.InitialMaxFlySpeed`) (`self.Character Movement`)))))

(fn `GetFloorResult`
  (locals (CharacterCurrentLocation :type "Vector Structure" :default (0.0 0.0 0.0)))
  (set `local.CharacterCurrentLocation` (`KismetMathLibrary.MakeVector` (.x (`Actor.K2_GetActorLocation` (`self.GetOwner`))) (.y (`Actor.K2_GetActorLocation` (`self.GetOwner`))) (- (.z (`Actor.K2_GetActorLocation` (`self.GetOwner`))) (`CapsuleComponent.CapsuleHalfHeight` (`self.Capsule Component`)))))
  (bind _outhit (`KismetSystemLibrary.LineTraceSingle` :`Start` (`local.CharacterCurrentLocation`) :`End` (+ (`local.CharacterCurrentLocation`) (* (`KismetMathLibrary.Vector_Down`) 5000.0)) :`TraceChannel` "TraceTypeQuery1" :`DrawDebugType` "ForOneFrame"))
  (bind _output_get (set `self.Out Hit` _outhit))
  (bind (_bblockinghit _binitialoverlap) (`GameplayStatics.BreakHitResult` _output_get))
  (if (and _bblockinghit (not _binitialoverlap))
    (set `self.IsFoundGroundHit` true)
    (else
      (set `self.IsFoundGroundHit` false))))

(fn `GetResultForce`
  (bind _supportingforce (`self.GetSupportingForce`))
  (set `self.ResultForce` (+ _supportingforce (* (`self.Grivity`) 2.0) (* (* (`Actor.GetActorForwardVector` (`self.GetOwner`)) 20000.0) (`self.MoveForwardScaleValue`)))))

(fn `GetSupportingForce`
  (returns (SupportingForce :type "Vector Structure"))
  (if (`self.IsFoundGroundHit`)
    (set `self.Normal` (`.ImpactNormal` (`GameplayStatics.BreakHitResult` (`self.Out Hit`))))
    (return (* (* (`self.normal`) (`KismetMathLibrary.Dot_VectorVector` (`self.Grivity`) (`self.normal`))) -1))
    (else
      ;[1 1 1] 默认返回重力的反方向
      (return (* (`self.Grivity`) -1)))))

(fn `InitData`
  (bind _returnvalue (`self.GetOwner`))
  (bind _componentowner (`self.ComponentOwner`))
  (`|ExecutionSequence`
    (:`then_0`
      (`/Engine/EditorBlueprintResources/StandardMacros.IsValid` _returnvalue
        (:`Is Valid`
          (set `self.ComponentOwner` _returnvalue))))
    (:`then_1`
      (`/Engine/EditorBlueprintResources/StandardMacros.IsValid` _componentowner
        (:`Is Valid`
          (bind _asbpi_ability_owner (cast `/Game/SnowBoardGame/Blueprints/Interface/BPI_AbilityOwner` _componentowner))
          (bind _output_get (set `self.As BPI Ability Owner` _asbpi_ability_owner))
          (bind _character (`/Game/SnowBoardGame/Blueprints/Interface/BPI_AbilityOwner.GetCharacter` _output_get))
          (bind _output_get_2 (set `self.Character` _character))
          (set `self.Capsule Component` (`Character.CapsuleComponent` _output_get_2))
          (bind _output_get_3 (set `self.Character Movement` (`Character.CharacterMovement` _output_get_2)))
          (set `self.InitialMaxFlySpeed` (`CharacterMovementComponent.MaxFlySpeed` _output_get_3)))))))

(fn `InitSetting`
  (bind _character_movement (`self.Character Movement`))
  (`|ExecutionSequence`
    (:`then_0`
      (`/Game/SnowBoardGame/Blueprints/Interface/BPI_AbilityOwner.SetMotionMode` (`self.As BPI Ability Owner`) "NewEnumerator1")
      (`CharacterMovementComponent.SetMovementMode` (`self.Character Movement`) "MOVE_Flying" 0)
      (`self.SetComponentTickEnabled` true)
      (set `CharacterMovementComponent.MaxFlySpeed` (`self.MaxFlySpeed`) _character_movement)
      (set `CharacterMovementComponent.bUseControllerDesiredRotation` false _character_movement)
      (set `CharacterMovementComponent.bOrientRotationToMovement` false _character_movement))
    (:`then_1`
      (`self.SetGravity`))))

(fn `MoveForward`
  (params (Aixs :type "Float (double-precision)"))
  (set `self.MoveForwardScaleValue` Aixs))

(fn `MoveRight`
  (params (Axis :type "Float (double-precision)"))
  (`|ExecutionSequence`
    (:`then_0`
      (set `self.RightAxisValue` Axis)
      (if (> (`local.Axis`) 0.0)
        (set `self.RightValue` (`CurveFloat.GetFloatValue` (`self.MoveRightScaleCurve`) (`local.Axis`)))
        (elif (< (`local.Axis`) 0.0)
          (set `self.RightValue` (* -1 (`CurveFloat.GetFloatValue` (`self.MoveRightScaleCurve`) (`KismetMathLibrary.Abs` (`local.Axis`)))))
          (else
            (set `self.RightValue` 0.0)))))
    (:`then_1`
      (set `self.MoveRightForce` (* (`KismetMathLibrary.Normal` (`KismetMathLibrary.GetRightVector` (`KismetMathLibrary.MakeRotFromX` (`MovementComponent.Velocity` (`self.Character Movement`))))) (* (`self.RightValue`) (* (`KismetMathLibrary.VSize` (`MovementComponent.Velocity` (`self.Character Movement`))) (/ (`self.MoveRightForceLength`) 2400.0))))))))

(fn `SetGravity`
  (set `self.Grivity` (* (* (`KismetMathLibrary.Vector_Down`) (`self.Gravity`)) (* (`CharacterMovementComponent.Mass` (`Actor.GetComponentByClass` (`self.GetOwner`) "/Script/Engine.CharacterMovementComponent")) 10.0))))

(fn `UpateCharacterState`
  (`|ExecutionSequence`
    (:`then_0`
      (`self.AdjustCharacterRotation`))))

(fn `UpdateMovement`
  (`|ExecutionSequence`
    (:`then_0`
      (`self.GetFloorResult`))
    (:`then_1`
      (`self.GetResultForce`))
    (:`then_2`
      (`self.UpdateResultForce`))
    (:`then_3`
      (`self.AddMovementInput`))))

(fn `UpdateResultForce`
  (set `self.MovementDirection` (+ (`self.ResultForce`) (`self.MoveRightForce`))))