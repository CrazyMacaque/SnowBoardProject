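; BP_Character is a playable character for the snowboard game that delegates movement input to a swappable ability.
; BeginPlay activates the BPACSkiing ability, and key 1 flip-flops between activating and deactivating it, starting with activate.
; Forward and right axes are forwarded as messages to the current Ability, while turn and look axes drive controller rotation directly.
; It also exposes itself and a settable MotionMode through simple accessors.
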(event `self.ReceiveBeginPlay`
  (bind _bpac_skiing (`self.BPAC_Skiing`))
  ;[1 1 1] SwitchMotionMode
  (`/Game/SnowBoardGame/Blueprints/Interface/BPI_Ability.DoActive` _bpac_skiing :!label _label)
  (set `self.Ability` _bpac_skiing))

(event `InputAxis|MoveRight`
  (params (AxisValue :type "Float (single-precision)"))
  (bind _ability (`self.Ability`))
  (`/Engine/EditorBlueprintResources/StandardMacros.IsValid` (`KismetSystemLibrary.Conv_InterfaceToObject` _ability)
    (:`Is Valid`
      (message `/Game/SnowBoardGame/Blueprints/Interface/BPI_Ability.InputAxis` (`KismetSystemLibrary.Conv_InterfaceToObject` _ability) "NewEnumerator2" AxisValue))))

(event `InputAxis|Turn` :overrideparent false
  (params (AxisValue :type "Float (single-precision)"))
  (`self.AddControllerYawInput` AxisValue))

(event `InputAxis|MoveForward`
  (params (AxisValue :type "Float (single-precision)"))
  (bind _ability (`self.Ability`))
  (`/Engine/EditorBlueprintResources/StandardMacros.IsValid` (`KismetSystemLibrary.Conv_InterfaceToObject` _ability)
    (:`Is Valid`
      (message `/Game/SnowBoardGame/Blueprints/Interface/BPI_Ability.InputAxis` (`KismetSystemLibrary.Conv_InterfaceToObject` _ability) "NewEnumerator1" AxisValue))))

(event `InputAxis|LookUp` :overrideparent false
  (params (AxisValue :type "Float (single-precision)"))
  (`self.AddControllerPitchInput` AxisValue))

(event `Key|One`
  (params (Key :type "Key Structure"))
  ;[1 1 1] SwitchMotionMode
  (:`Pressed`
    (`/Engine/EditorBlueprintResources/StandardMacros.FlipFlop`
      (:`A`
        (goto _label))
      (:`B`
        (`/Game/SnowBoardGame/Blueprints/Interface/BPI_Ability.DoDeactive` (`self.BPAC_Skiing`))
        (set `self.Ability` null)))))

(event `/Game/SnowBoardGame/Blueprints/Interface/BPI_AbilityOwner.SetMotionMode`
  (params (motion :type "/Game/SnowBoardGame/Animations/UE/Enum/E_MotionMode Enum" :default "NewEnumerator0"))
  (set `self.MotionMode` motion))

(fn `GetCharacter`
  (returns (Character :type "Character Object Reference"))
  (return self))

(fn `GetMotionMode`
  (returns (Result :type "/Game/SnowBoardGame/Animations/UE/Enum/E_MotionMode Enum"))
  (return (`self.MotionMode`)))

(fn `UserConstructionScript`)