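; Blueprint function library that evaluates a point on a Catmull-Rom spline from four control points, a tension Γ and a parameter U.
; GetCatmullRom clamps Γ to 0–1 and builds the cubic coefficients through GetC0 to GetC3.
; GetCurvePoints evaluates that polynomial at an unclamped U, with 0 to 1 spanning the second to third control point.
; CatmullRomFunc is an unfinished stub whose GetCatmullRom call is never executed.
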(fn `CatmullRomFunc`
  (params (ContolPoints1 :type "Vector Structure") (ContolPoints2 :type "Vector Structure") (ContolPoints3 :type "Vector Structure") (ContolPoints4 :type "Vector Structure") (`γ` :type "Float (double-precision)") (U :type "Vector Structure")))

(fn `GetC0`
  (params (ContolPoints2 :type "Vector Structure"))
  (returns (C0 :type "Vector Structure"))
  (return ContolPoints2))

(fn `GetC1`
  (params (ControlPoints1 :type "Vector Structure") (ControlPoints3 :type "Vector Structure") (`γ` :type "Float (double-precision)"))
  (returns (C1 :type "Vector Structure"))
  (return (+ (* ControlPoints3 `γ`) (* ControlPoints1 (* -1 `γ`)))))

(fn `GetC2`
  (params (ContolPoints1 :type "Vector Structure") (ContolPoints2 :type "Vector Structure") (ContolPoints3 :type "Vector Structure") (ContolPoints4 :type "Vector Structure") (`γ` :type "Float (double-precision)"))
  (returns (C2 :type "Vector Structure"))
  (bind _returnvalue (* 2 `γ`))
  (return (+ (* ContolPoints1 _returnvalue) (* ContolPoints2 (- `γ` 3.0)) (* ContolPoints3 (- 3.0 _returnvalue)) (* ContolPoints4 (* -1 `γ`)))))

(fn `GetC3`
  (params (ContolPoints1 :type "Vector Structure") (ContolPoints2 :type "Vector Structure") (ContolPoints3 :type "Vector Structure") (ContolPoints4 :type "Vector Structure") (`γ` :type "Float (double-precision)"))
  (returns (C3 :type "Vector Structure"))
  (return (+ (* ContolPoints1 (* -1 `γ`)) (* ContolPoints2 (- 2.0 `γ`)) (* ContolPoints3 (- `γ` 2.0)) (* ContolPoints4 `γ`))))

(fn `GetCatmullRom`
  (params (ContolPoints1 :type "Vector Structure") (ContolPoints2 :type "Vector Structure") (ContolPoints3 :type "Vector Structure") (ContolPoints4 :type "Vector Structure") (`γ` :type "Float (double-precision)") (U :type "Vector Structure"))
  (returns (CurvePoint :type "Vector Structure"))
  (bind _returnvalue (`KismetMathLibrary.FClamp` `γ`))
  (bind _c0 (`self.GetC0` ContolPoints2))
  (bind _c1 (`self.GetC1` ContolPoints1 ContolPoints3 _returnvalue))
  (bind _c2 (`self.GetC2` ContolPoints1 ContolPoints2 ContolPoints3 ContolPoints4 _returnvalue))
  (bind _c3 (`self.GetC3` ContolPoints1 ContolPoints2 ContolPoints3 ContolPoints4 _returnvalue))
  (bind _curvepoint (`self.GetCurvePoints` _c0 _c1 _c2 _c3 U))
  (return _curvepoint))

(fn `GetCurvePoints`
  (params (C0 :type "Vector Structure") (C1 :type "Vector Structure") (C2 :type "Vector Structure") (C3 :type "Vector Structure") (U :type "Vector Structure"))
  (returns (CurvePoint :type "Vector Structure"))
  (return (+ C0 (* C1 U) (* C2 U U) (* C3 U U U))))