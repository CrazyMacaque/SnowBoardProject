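; Blueprint function library in the snowboard game for evaluating Bezier curves and shaping splines from them.
; BezierCurve recursively lerps control points (De Casteljau) for any point count, while EasyBezierCurve uses the closed-form quadratic formula.
; UseBezierCurveWithSpline converts actor-local control points to world space, samples the curve behind a CanUpdate guard, and projects samples via GetTrackPoints.
; It writes the projected points to the spline and returns them with impact normals.
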(fn `Bezier Curve`
  (params (VectorArray :type "Array of Vector Structure") (t :type "Float (double-precision)"))
  (returns (Output :type "Vector Structure (by ref)"))
  (locals (TempLocalVar :type "Array of Vector Structure"))
  (bind _returnvalue (`KismetArrayLibrary.Array_Length` VectorArray))
  (if (<= _returnvalue 1)
    (return (`|GetArrayItem` VectorArray))
    (else
      (for _index (range (+ (- _returnvalue 2) 1))
        (`KismetArrayLibrary.Array_Add` (`local.TempLocalVar`) (`KismetMathLibrary.VLerp` (`|GetArrayItem` VectorArray _index) (`|GetArrayItem` VectorArray (+ _index 1)) t)))
      (bind _output (`self.Bezier Curve` (`local.TempLocalVar`) t))
      (return _output))))

(fn `EasyBezierCurve`
  (params (Start :type "Vector Structure") (ControlPoint :type "Vector Structure") (End :type "Vector Structure") (t :type "Float (double-precision)"))
  (returns (ReturnValue :type "Vector Structure"))
  (locals (`1-t` :type "Float (double-precision)" :default 0.0))
  (set `local.1-t` (- 1.0 t))
  (return (+ (* Start (`KismetMathLibrary.Square` (`local.1-t`))) (* ControlPoint (* (`local.1-t`) 2.0 t)) (* End (`KismetMathLibrary.Square` t)))))

(fn `UseBezierCurveWithSpline`
  (params (ControlPointsArray :type "Array of Vector Structure") (Spline :type "SplineComponent Object Reference") (SelfActor :type "Actor Object Reference"))
  (returns (CurvePointsArray :type "Array of Vector Structure") (ImpactNormal1 :type "Array of Vector Structure"))
  (locals (TempCurvePoints :type "Array of Vector Structure") (T :type "Float (double-precision)") (SplinePoints :type "Array of Vector Structure") (`Last Index` :type Integer :default 50) (CanUpdate :type Boolean :default true) (TempSplinePoints :type "Array of Vector Structure"))
  (if (`local.CanUpdate`)
    ;[0.04817 0.4452 0.8632] 将本地坐标转换为世界坐标
    (for _array_element ControlPointsArray
      (`KismetArrayLibrary.Array_Add` (`local.TempCurvePoints`) (`KismetMathLibrary.TransformLocation` (`Actor.GetTransform` SelfActor) _array_element)))
    ;[0.2384 0.06125 0.8714] 计算贝塞尔曲线点
    (for _ (range (`local.Last Index`))
      (set `local.CanUpdate` false)
      (bind _output (`self.Bezier Curve` (`local.TempCurvePoints`) (`local.T`)))
      (set `local.T` (+ (`local.T`) (/ 1.0 (`KismetMathLibrary.Conv_IntToDouble` (`local.Last Index`)))))
      (`KismetArrayLibrary.Array_Add` (`local.TempSplinePoints`) _output))
    (set `local.CanUpdate` true)
    ;[0.07036 0.3325 0.8714] 将目标曲线点转换为投影点
    (bind (_newparam _impactnormal1) (`/Game/SnowBoardGame/Blueprints/FunctionLibrary/BPF_TrackDrawing.GetTrackPoints` (`local.TempSplinePoints`)))
    ;[0.2747 0.5972 0.9216] 设置样条线
    (`SplineComponent.SetSplinePoints` Spline _newparam "World" true)
    (return _newparam _impactnormal1)))