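; Track-drawing function library for the snowboard game that projects curve points onto the static world geometry beneath them.
; GetTrackPoints line-traces straight down by TraceLength from each target point against WorldStatic objects.
; It returns parallel arrays of hit locations and impact normals, dropping points that miss, so the output can be shorter than the input.
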(fn `GetTrackPoints`
  (params (TargetPoints :type "Array of Vector Structure"))
  (returns (NewParam :type "Array of Vector Structure") (ImpactNormal1 :type "Array of Vector Structure"))
  (locals (TraceLength :type "Float (double-precision)" :default 5000.0) (TracePoints :type "Array of Vector Structure") (ImpactNormal :type "Array of Vector Structure"))
  (for _array_element TargetPoints
    (bind (_outhit _returnvalue) (`KismetSystemLibrary.LineTraceSingleForObjects` null _array_element (+ _array_element (* (`KismetMathLibrary.Vector_Down`) (`local.TraceLength`))) (`|MakeArray` "ObjectTypeQuery1" :!type "EObjectTypeQuery Enum") false (`|MakeArray` null :!type "Actor Object Reference")))
    (if _returnvalue
      (bind (_bblockinghit _binitialoverlap _time _distance _location _impactpoint _normal _impactnormal) (`GameplayStatics.BreakHitResult` _outhit))
      (`KismetArrayLibrary.Array_Add` (`local.TracePoints`) _location)
      (`KismetArrayLibrary.Array_Add` (`local.ImpactNormal`) _impactnormal)))
  (return (`local.TracePoints`) (`local.ImpactNormal`)))